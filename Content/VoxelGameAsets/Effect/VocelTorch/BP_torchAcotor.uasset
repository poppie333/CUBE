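; Torch actor with a Niagara effect and a point light that switches on or off with the player's era state.
; It caches the player pawn as PlayerCharacterBP on BeginPlay, then polls its EraChange flag every Tick.
; When the flag is set, the effect is hidden, its collision response becomes Overlap and the light goes dark.
; Otherwise the effect is visible and blocking, and the light is lit.
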(event `self.ReceiveBeginPlay`
  (bind _asplayer_character_bp (cast `/Game/BluePrint/PlayerCharacterBP` (`GameplayStatics.GetPlayerPawn` 0))))

(event `self.ReceiveTick`
  (params (DeltaSeconds :type "Float (single-precision)"))
  (bind _niagara (`self.Niagara`))
  (bind _pointlight (`self.PointLight`))
  (if (`/Game/BluePrint/PlayerCharacterBP.EraChange` (stale `self.ReceiveBeginPlay` _asplayer_character_bp))
    (`SceneComponent.SetVisibility` _niagara false false)
    (`PrimitiveComponent.SetCollisionResponseToAllChannels` _niagara "ECR_Overlap")
    (`LightComponent.SetIntensity` _pointlight 0.0)
    (else
      (`SceneComponent.SetVisibility` _niagara true false)
      (`PrimitiveComponent.SetCollisionResponseToAllChannels` _niagara "ECR_Block")
      (`LightComponent.SetIntensity` _pointlight 2096.986816))))

(fn `UserConstructionScript`)