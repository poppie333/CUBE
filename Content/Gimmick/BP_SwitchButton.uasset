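; BP_SwitchButton is a gimmick switch that lowers the elevator when the player steps into its Box trigger.
; On overlap it finds BP_ElevatorGimmick and the BP_GetCoordinates marker, then Tick moves the elevator toward the marker by a fixed, frame-rate-dependent step.
; A four-second Delay in Tick stops the movement and sets the elevator's GimmickON.
; Tick also disables the trigger's collision while the player's EraChange flag is set.
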(event `self.ReceiveBeginPlay`
  ;[1 1 1] 初期化
  (set `self.SwitchON` false)
  (set `self.velocity` 2.4)
  (bind _asplayer_character_bp (cast `/Game/BluePrint/PlayerCharacterBP` (`GameplayStatics.GetPlayerPawn` 0))))

(event `self.ReceiveTick`
  (params (DeltaSeconds :type "Float (single-precision)"))
  (bind _box (`self.Box`))
  ;[1 1 1] エレベーターと座標取得のアクターの座標をベクトル化し、エレベーターが指定座標まで降下し続ける
  (if (`/Game/BluePrint/PlayerCharacterBP.EraChange` (stale `self.ReceiveBeginPlay` _asplayer_character_bp))
    (`PrimitiveComponent.SetCollisionEnabled` _box "NoCollision")
    (else
      (`PrimitiveComponent.SetCollisionEnabled` _box "QueryOnly")))
  (if (`self.SwitchON`)
    (`self.K2_AddActorWorldOffset` (stale `self.Box.OnComponentBeginOverlap` _returnvalue) (* (* (`KismetMathLibrary.Normal` (- (`self.K2_GetActorLocation` (stale `self.Box.OnComponentBeginOverlap` _returnvalue)) (`self.K2_GetActorLocation` (stale `self.Box.OnComponentBeginOverlap` _returnvalue_2)))) (`self.velocity`)) (-1.0 -1.0 -1.0)) false false)
    (`KismetSystemLibrary.Delay` 4.0)
    (set `self.SwitchON` false)
    (set `/Game/Gimmick/GimmickCube/BP_ElevatorGimmick.GimmickON` true (stale `self.Box.OnComponentBeginOverlap` _returnvalue))))

(event `self.Box.OnComponentBeginOverlap`
  (params (OverlappedComponent :type "PrimitiveComponent Object Reference") (OtherActor :type "Actor Object Reference") (OtherComp :type "PrimitiveComponent Object Reference") (OtherBodyIndex :type Integer) (bFromSweep :type Boolean) (SweepResult :type "HitResult Structure (by ref)"))
  ;[1 1 1] Boxコリジョンに触れたのがプレイヤーの場合、エレベーターと座標取得のアクターを探し、SwitchONフラグを有効にする
  (if (== OtherActor (`GameplayStatics.GetPlayerCharacter` 0))
    (bind _returnvalue (`GameplayStatics.GetActorOfClass` "/Game/Gimmick/GimmickCube/BP_ElevatorGimmick.BP_ElevatorGimmick_C"))
    (bind _returnvalue_2 (`GameplayStatics.GetActorOfClass` "/Game/Gimmick/BP_GetCoordinates.BP_GetCoordinates_C"))
    (set `self.SwitchON` true)))

(fn `UserConstructionScript`)