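; Elevator gimmick actor that carries the player vertically between its start height and a fixed height above it.
; Overlapping the Box starts movement and leaving stops it; Tick applies a fixed per-frame offset, not scaled by delta time.
; Passing either endpoint reverses direction and halts until the next overlap.
; While the player's EraChange flag is set, movement pauses and the mesh is hidden with overlap-only collision.
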(event `self.ReceiveBeginPlay`
  (bind (_returnvalue_x _returnvalue_y _returnvalue_z) (`KismetMathLibrary.BreakVector` (`self.K2_GetActorLocation`)))
  ;[1 1 1] スタート地点と折り返し地点を取得
  (set `self.EndLocationZ` (+ _returnvalue_z 710.0))
  (set `self.StartLocationZ` _returnvalue_z)
  (set `self.GimmickON` false)
  (bind _asplayer_character_bp (cast `/Game/BluePrint/PlayerCharacterBP` (`GameplayStatics.GetPlayerPawn` 0))))

(event `self.ReceiveTick`
  (params (DeltaSeconds :type "Float (single-precision)"))
  (bind (_returnvalue_x _returnvalue_y _returnvalue_z) (`KismetMathLibrary.BreakVector` (`self.K2_GetActorLocation`)))
  (bind (_returnvalue_x_2 _returnvalue_y_2 _returnvalue_z_2) (`KismetMathLibrary.BreakVector` (`self.K2_GetActorLocation`)))
  (bind _sm_elevator (`self.SM_elevator`))
  ;[1 1 1] エレベーターの往復移動処理
  (if (`/Game/BluePrint/PlayerCharacterBP.EraChange` (stale `self.ReceiveBeginPlay` _asplayer_character_bp))
    (`SceneComponent.SetVisibility` _sm_elevator false false)
    (`PrimitiveComponent.SetCollisionResponseToAllChannels` _sm_elevator "ECR_Overlap")
    (else
      (`SceneComponent.SetVisibility` _sm_elevator true false)
      (`PrimitiveComponent.SetCollisionResponseToAllChannels` _sm_elevator "ECR_Block")
      (if (`self.GimmickON`)
        (`self.K2_AddActorLocalOffset` (`self.ElevatorLocation`))
        (if (> _returnvalue_z_2 (`self.EndLocationZ`))
          (set `self.ElevatorLocation` (0.0 0.0 -2.4))
          (set `self.GimmickON` false)
          (elif (< _returnvalue_z (`self.StartLocationZ`))
            (set `self.ElevatorLocation` (0.0 0.0 2.4))
            (set `self.GimmickON` false)))))))

(event `self.Box.OnComponentBeginOverlap`
  (params (OverlappedComponent :type "PrimitiveComponent Object Reference") (OtherActor :type "Actor Object Reference") (OtherComp :type "PrimitiveComponent Object Reference") (OtherBodyIndex :type Integer) (bFromSweep :type Boolean) (SweepResult :type "HitResult Structure (by ref)"))
  ;[1 1 1] コリジョンに触れたら起動、離れたら停止する処理
  (if (== OtherActor (`GameplayStatics.GetPlayerCharacter` 0))
    (set `self.GimmickON` true)))

(event `self.Box.OnComponentEndOverlap`
  (params (OverlappedComponent :type "PrimitiveComponent Object Reference") (OtherActor :type "Actor Object Reference") (OtherComp :type "PrimitiveComponent Object Reference") (OtherBodyIndex :type Integer))
  ;[1 1 1] コリジョンに触れたら起動、離れたら停止する処理
  (if (== OtherActor (`GameplayStatics.GetPlayerCharacter` 0))
    (set `self.GimmickON` false)))

(fn `UserConstructionScript`)