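; BP_LadderGimmick01 is a ladder gimmick that lifts the player upward when they touch its Box trigger.
; An overlap by the player character sets LadderBool, and the next Tick teleports the player up along local Z without sweep, then clears the flag.
; Tick also reads EraChange from the cached PlayerCharacterBP, disabling Box collision while it is true and restoring query-only collision otherwise.
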(event `self.ReceiveBeginPlay`
  (bind _asplayer_character_bp (cast `/Game/BluePrint/PlayerCharacterBP` (`GameplayStatics.GetPlayerCharacter` 0))))

(event `self.ReceiveTick`
  (params (DeltaSeconds :type "Float (single-precision)"))
  (bind _box (`self.Box`))
  (if (`/Game/BluePrint/PlayerCharacterBP.EraChange` (stale `self.ReceiveBeginPlay` _asplayer_character_bp))
    (`PrimitiveComponent.SetCollisionEnabled` _box "NoCollision")
    (else
      (`PrimitiveComponent.SetCollisionEnabled` _box "QueryOnly")))
  (if (`self.LadderBool`)
    (`self.K2_AddActorLocalOffset` (`GameplayStatics.GetPlayerCharacter` 0) (0.0 0.0 100.0) false true)
    (set `self.LadderBool` false)))

(event `self.Box.OnComponentBeginOverlap`
  (params (OverlappedComponent :type "PrimitiveComponent Object Reference") (OtherActor :type "Actor Object Reference") (OtherComp :type "PrimitiveComponent Object Reference") (OtherBodyIndex :type Integer) (bFromSweep :type Boolean) (SweepResult :type "HitResult Structure (by ref)"))
  (if (== OtherActor (`GameplayStatics.GetPlayerCharacter` 0))
    (set `self.LadderBool` true)))

(fn `UserConstructionScript`)