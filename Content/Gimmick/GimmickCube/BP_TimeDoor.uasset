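; Time door gimmick that moves the actor along a per-tick local offset, like an elevator, once the player character overlaps its Box.
; BeginPlay records the starting Z and an end Z 200 units above it, and the overlap sets GimmickON.
; Tick applies the unswept offset until Z leaves that range, then stops, resetting the offset upward if below the start.
; The downward-offset node is unconnected, and no end-overlap stop exists.
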(event `self.ReceiveBeginPlay`
  (bind (_returnvalue_x _returnvalue_y _returnvalue_z) (`KismetMathLibrary.BreakVector` (`self.K2_GetActorLocation`)))
  ;[1 1 1] スタート地点と折り返し地点を取得
  (set `self.EndLocationZ` (+ _returnvalue_z 200.0))
  (set `self.StartLocationZ` _returnvalue_z)
  (set `self.GimmickON` false))

(event `self.ReceiveTick`
  (params (DeltaSeconds :type "Float (single-precision)"))
  (bind (_returnvalue_x _returnvalue_y _returnvalue_z) (`KismetMathLibrary.BreakVector` (`self.K2_GetActorLocation`)))
  (bind (_returnvalue_x_2 _returnvalue_y_2 _returnvalue_z_2) (`KismetMathLibrary.BreakVector` (`self.K2_GetActorLocation`)))
  ;[1 1 1] エレベーターの往復移動処理
  (if (`self.GimmickON`)
    (`self.K2_AddActorLocalOffset` (`self.ElevatorLocation`))
    (if (> _returnvalue_z_2 (`self.EndLocationZ`))
      (set `self.GimmickON` false :!label _label)
      (elif (< _returnvalue_z (`self.StartLocationZ`))
        (set `self.ElevatorLocation` (0.0 0.0 0.05))
        (goto _label)))))

(event `self.Box.OnComponentBeginOverlap`
  (params (OverlappedComponent :type "PrimitiveComponent Object Reference") (OtherActor :type "Actor Object Reference") (OtherComp :type "PrimitiveComponent Object Reference") (OtherBodyIndex :type Integer) (bFromSweep :type Boolean) (SweepResult :type "HitResult Structure (by ref)"))
  ;[1 1 1] コリジョンに触れたら起動、離れたら停止する処理
  (if (== OtherActor (`GameplayStatics.GetPlayerCharacter` 0))
    (set `self.GimmickON` true)))

(fn `UserConstructionScript`)