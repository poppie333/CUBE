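; BP_Button is a gimmick pressure button that visually sinks when the player character steps on it.
; Box overlap begin and end events lower and raise the SMButton02 mesh with local offsets, with no other effect triggered.
; Tick reads EraChange from the cached PlayerCharacterBP and swaps collision responses: when true, Box blocks and both meshes overlap; when false, Box overlaps and both meshes block.
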(event `self.Box.OnComponentBeginOverlap`
  (params (OverlappedComponent :type "PrimitiveComponent Object Reference") (OtherActor :type "Actor Object Reference") (OtherComp :type "PrimitiveComponent Object Reference") (OtherBodyIndex :type Integer) (bFromSweep :type Boolean) (SweepResult :type "HitResult Structure (by ref)"))
  ;[1 1 1] buttonが押されたときの挙動
  (if (== OtherActor (`GameplayStatics.GetPlayerCharacter` 0))
    (`SceneComponent.K2_AddLocalOffset` (`self.SM_button02`) (0.0 0.0 -6.0) false false)))

(event `self.Box.OnComponentEndOverlap`
  (params (OverlappedComponent :type "PrimitiveComponent Object Reference") (OtherActor :type "Actor Object Reference") (OtherComp :type "PrimitiveComponent Object Reference") (OtherBodyIndex :type Integer))
  ;[1 1 1] buttonが押されたときの挙動
  (if (== OtherActor (`GameplayStatics.GetPlayerCharacter` 0))
    (`SceneComponent.K2_AddLocalOffset` (`self.SM_button02`) (0.0 0.0 6.0) false false)))

(event `self.ReceiveBeginPlay`
  (bind _asplayer_character_bp (cast `/Game/BluePrint/PlayerCharacterBP` (`GameplayStatics.GetPlayerCharacter` 0))))

(event `self.ReceiveTick`
  (params (DeltaSeconds :type "Float (single-precision)"))
  (bind _box (`self.Box`))
  (bind _sm_button02 (`self.SM_button02`))
  (bind _sm_button01 (`self.SM_button01`))
  (if (`/Game/BluePrint/PlayerCharacterBP.EraChange` (stale `self.ReceiveBeginPlay` _asplayer_character_bp))
    (`PrimitiveComponent.SetCollisionResponseToAllChannels` _box "ECR_Block")
    (`PrimitiveComponent.SetCollisionResponseToAllChannels` _sm_button02 "ECR_Overlap")
    (`PrimitiveComponent.SetCollisionResponseToAllChannels` _sm_button01 "ECR_Overlap")
    (else
      (`PrimitiveComponent.SetCollisionResponseToAllChannels` _box "ECR_Overlap")
      (`PrimitiveComponent.SetCollisionResponseToAllChannels` _sm_button02 "ECR_Block")
      (`PrimitiveComponent.SetCollisionResponseToAllChannels` _sm_button01 "ECR_Block"))))

(fn `UserConstructionScript`)