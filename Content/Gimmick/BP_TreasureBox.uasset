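; BP_TreasureBox is a treasure chest gimmick that exists only while the player's EraChange flag is false.
; Tick reads that flag each frame, toggling chest and light visibility and switching mesh collision between Overlap and Block.
; Player overlap on Box_Lid rotates the lid pivot open.
; Overlap on Box waits briefly, hides the light (which Tick can re-show), and sets OnTreasure once.
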(event `self.ReceiveBeginPlay`
  (set `self.OnTreasure` false)
  (bind _asplayer_character_bp (cast `/Game/BluePrint/PlayerCharacterBP` (`GameplayStatics.GetPlayerCharacter` 0))))

(event `self.ReceiveTick`
  (params (DeltaSeconds :type "Float (single-precision)"))
  (bind _sm_treasurechesta (`self.SM_TreasureChestA`))
  (if (`/Game/BluePrint/PlayerCharacterBP.EraChange` (stale `self.ReceiveBeginPlay` _asplayer_character_bp))
    (`SceneComponent.SetVisibility` (`self.SM_TreasureChestB`) false false)
    (`SceneComponent.SetVisibility` _sm_treasurechesta false false)
    (`SceneComponent.SetVisibility` (`self.PointLight`) false false)
    (`PrimitiveComponent.SetCollisionResponseToAllChannels` _sm_treasurechesta "ECR_Overlap")
    (`PrimitiveComponent.SetCollisionResponseToAllChannels` (`self.SM_TreasureChestB`) "ECR_Overlap")
    (else
      (`SceneComponent.SetVisibility` _sm_treasurechesta true false)
      (`SceneComponent.SetVisibility` (`self.SM_TreasureChestB`) true false)
      (`SceneComponent.SetVisibility` (`self.PointLight`) true false)
      (`PrimitiveComponent.SetCollisionResponseToAllChannels` _sm_treasurechesta "ECR_Block")
      (`PrimitiveComponent.SetCollisionResponseToAllChannels` (`self.SM_TreasureChestB`) "ECR_Block"))))

(event `self.Box.OnComponentBeginOverlap`
  (params (OverlappedComponent :type "PrimitiveComponent Object Reference") (OtherActor :type "Actor Object Reference") (OtherComp :type "PrimitiveComponent Object Reference") (OtherBodyIndex :type Integer) (bFromSweep :type Boolean) (SweepResult :type "HitResult Structure (by ref)"))
  (if (== OtherActor (`GameplayStatics.GetPlayerCharacter` 0))
    (`KismetSystemLibrary.Delay` 1.5)
    (`SceneComponent.SetVisibility` (`self.PointLight`) false false)
    (`/Engine/EditorBlueprintResources/StandardMacros.DoOnce` false
      (:`Completed`
        (set `self.OnTreasure` true)))))

(event `self.Box_Lid.OnComponentBeginOverlap`
  (params (OverlappedComponent :type "PrimitiveComponent Object Reference") (OtherActor :type "Actor Object Reference") (OtherComp :type "PrimitiveComponent Object Reference") (OtherBodyIndex :type Integer) (bFromSweep :type Boolean) (SweepResult :type "HitResult Structure (by ref)"))
  (if (== OtherActor (`GameplayStatics.GetPlayerCharacter` 0))
    (set `self.Box Open` true)
    (`self.Rotate Box Lid`)))

(fn `Rotate Box Lid`
  (if (`self.Box Open`)
    (`SceneComponent.K2_SetRelativeRotation` (`self.Lid Pivot`) (struct :`Roll` 90.0) false false)))

(fn `UserConstructionScript`)