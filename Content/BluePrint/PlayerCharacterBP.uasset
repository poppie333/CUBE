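; Player character Blueprint with automatic ladder climbing and an input-driven era toggle.
; Capsule overlaps with actors tagged Ladder set OnLadder and switch movement between Flying and Walking, while Tick lifts the character by a fixed local offset per frame, without input or sweep.
; The generation-change Enhanced Input action spawns an attached Niagara fade effect and flips EraChange, which this graph never otherwise uses.
; A debug key prints a test string.
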(event OnComponentEndOverlap(CapsuleComponent)
  (params (OverlappedComponent :type Primitive%20Component%20Object%20Reference) (OtherActor :type Actor%20Object%20Reference) (OtherComp :type Primitive%20Component%20Object%20Reference) (OtherBodyIndex :type Integer))
  (if (Actor|ActorHasTag OtherActor "Ladder")
    (Variables|Default|SetOnLadder false)
    (Pawn|Components|CharacterMovement|SetMovementMode (Variables|Character|GetCharacterMovement) "MOVE_Walking" 0)))

(event OnComponentBeginOverlap(CapsuleComponent)
  (params (OverlappedComponent :type Primitive%20Component%20Object%20Reference) (OtherActor :type Actor%20Object%20Reference) (OtherComp :type Primitive%20Component%20Object%20Reference) (OtherBodyIndex :type Integer) (bFromSweep :type Boolean) (SweepResult :type Hit%20Result%20Structure%20%28by%20ref%29))
  (if (Actor|ActorHasTag OtherActor "Ladder")
    (Variables|Default|SetOnLadder true)
    (Pawn|Components|CharacterMovement|SetMovementMode (Variables|Character|GetCharacterMovement) "MOVE_Flying" 0)))

(event Input|EnhancedActionEvents|EnhancedInputActionIA_CharacterGenerationChange
  (params (ActionValue :type Vector%202D%20Structure) (ElapsedSeconds :type Float%20%28double-precision%29) (TriggeredSeconds :type Float%20%28double-precision%29) (InputAction :type Input%20Action%20Object%20Reference :default "/Game/Input/InputAction/IA_CharacterGenerationChange.IA_CharacterGenerationChange"))
  (:Started
    (Niagara|SpawnSystemAttached "/Game/VoxelGameAsets/Effect/fadeEffect/NS_FadeEffect.NS_FadeEffect" (Variables|Default|GetNiagara) "None" "0, 0, 0" "0, 0, 0" "KeepRelativeOffset" false)
    (if (Variables|Default|GetEraChange)
      (Variables|Default|SetEraChange false)
      (else
        (Variables|Default|SetEraChange true)))))

(event EventTick
  (params (DeltaSeconds :type Float%20%28single-precision%29))
  (if (Variables|Default|GetOnLadder)
    (Transformation|AddActorLocalOffset "0.000000,0.000000,10.000000" false false)))

(event Input|KeyboardEvents|DebugKeyT
  (params (Key :type Key%20Structure :default "None") (ActionValue :type Input%20Action%20Value%20Structure))
  (:Pressed
    (Development|PrintString "Hello")))

(fn ConstructionScript)