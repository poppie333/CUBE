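; Title-screen Blueprint that, judging by its name, plays a Game Boy power-on effect by revealing and sliding a Widget component.
; The widget is hidden on BeginPlay and its starting relative Y is cached.
; Once IsPressed is true, which nothing in this graph sets, Tick shows the widget and lowers Y by a fixed per-frame step, moving it only while the value stays above zero.
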(event `self.ReceiveBeginPlay`
  (bind _widget (`self.Widget`))
  (bind (_relativelocation_x _relativelocation_y) (`KismetMathLibrary.BreakVector` (`SceneComponent.RelativeLocation` _widget)))
  (`SceneComponent.SetVisibility` _widget false false)
  (set `self.NewLocation` _relativelocation_y))

(event `self.ReceiveTick`
  (params (DeltaSeconds :type "Float (single-precision)"))
  (if (`self.IsPressed`)
    (`SceneComponent.SetVisibility` (`self.Widget`) true false)
    (bind _output_get (set `self.NewLocation` (- (`self.NewLocation`) 1.0)))
    (if (> _output_get 0.0)
      (`SceneComponent.K2_SetRelativeLocation` (`self.Widget`) (`KismetMathLibrary.MakeVector` 0.0 (`self.NewLocation`)) false false))))

(fn `UserConstructionScript`)